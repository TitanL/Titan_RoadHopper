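; BP_Player is a player Blueprint with body and head meshes and a rudimentary keyboard-triggered move.
; The construction script assigns BodyModel and HeadModel to the Body and Head components.
; BeginPlay's MovePlayer event and the W press share a keyboard-key check on the W event's Key output.
; When it passes, MoveComponentTo sends DefaultSceneRoot to a fixed location on the Y axis, rather than offsetting it per press.
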(event Custom|MovePlayer
  (if (Class|KismetInputLibrary|KeyIsKeyboardKey (stale Input|KeyboardEvents|W Key))
    (Components|MoveComponentTo (Variables|Default|GetDefaultSceneRoot) "0,100.000000, 0" "0, 0, 0" false false 0.2 false)))

(event EventBeginPlay
  (CallFunction|MovePlayer))

(event Collision|EventActorBeginOverlap
  (params (OtherActor :type Actor%20Object%20Reference)))

(event EventTick
  (params (DeltaSeconds :type Float%20%28single-precision%29)))

(event Input|KeyboardEvents|W
  (params (Key :type Key%20Structure :default "None"))
  (:Pressed
    (if (Class|KismetInputLibrary|KeyIsKeyboardKey Key)
      (Components|MoveComponentTo (Variables|Default|GetDefaultSceneRoot) "0,100.000000, 0" "0, 0, 0" false false 0.2 false))))

(fn ConstructionScript
  (Components|StaticMesh|SetStaticMesh (Variables|Default|GetBody) (Variables|Default|GetBodyModel))
  (Components|StaticMesh|SetStaticMesh (Variables|Default|GetHead) (Variables|Default|GetHeadModel)))